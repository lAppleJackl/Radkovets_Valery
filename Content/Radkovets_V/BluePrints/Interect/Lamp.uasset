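; Lamp actor whose point light cycles endlessly through magenta, blue and green.
; BeginPlay enters a chain of latent Delay nodes, each holding for two seconds before the next SetLightColor call.
; The chain ends by calling its own Repeat custom event, forming a timed loop without Tick or a timeline, with hard color switches rather than blends.
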(event Custom|Repeat
  (Utilities|FlowControl|Delay 2.0)
  (Rendering|Components|Light|SetLightColor (Variables|Default|GetPointLight) "(R=1.000000,G=0.000000,B=0.975798,A=1.000000)" true)
  (Utilities|FlowControl|Delay 2.0)
  (Rendering|Components|Light|SetLightColor (Variables|Default|GetPointLight) "(R=0.000000,G=0.082511,B=1.000000,A=1.000000)" true)
  (Utilities|FlowControl|Delay 2.0)
  (Rendering|Components|Light|SetLightColor (Variables|Default|GetPointLight) "(R=0.000000,G=1.000000,B=0.081037,A=1.000000)" true)
  (CallFunction|Repeat))

(event EventBeginPlay
  (Utilities|FlowControl|Delay 2.0)
  (Rendering|Components|Light|SetLightColor (Variables|Default|GetPointLight) "(R=1.000000,G=0.000000,B=0.975798,A=1.000000)" true)
  (Utilities|FlowControl|Delay 2.0)
  (Rendering|Components|Light|SetLightColor (Variables|Default|GetPointLight) "(R=0.000000,G=0.082511,B=1.000000,A=1.000000)" true)
  (Utilities|FlowControl|Delay 2.0)
  (Rendering|Components|Light|SetLightColor (Variables|Default|GetPointLight) "(R=0.000000,G=1.000000,B=0.081037,A=1.000000)" true)
  (CallFunction|Repeat))

(fn ConstructionScript)