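; MainCharacter is a player character Blueprint with basic movement, mouse-look style turning and hold-to-sprint.
; Input axes drive movement along the actor's forward and right vectors and add controller yaw and pitch.
; The Speed action switches MaxWalkSpeed to HighSpeed while held and restores Speed on release, with no gradual acceleration.
; The Interact action only prints debug strings on press and release.
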(event Input|ActionEvents|InputActionInteract
  (params (Key :type Key%20Structure :default "None"))
  ;[1 1 1] То что было на уроке
  (:Pressed
    (Development|PrintString "Press E"))
  (:Released
    (Development|PrintString "Repress E")))

(event Input|ActionEvents|InputActionSpeed
  (params (Key :type Key%20Structure :default "None"))
  (bind _charactermovement (Variables|Character|GetCharacterMovement))
  ;[1 1 1] ДЗ на ускорение через SHIFT, хотел ещё сделать ускорение постепенное, игрок зажимает клавишу W и каждую секунду прибавляется 50 к скорости до определённого лимита, как только он её отпускает, скорость возврашяется к стандартной, но так и не разобрался как это сделать на blueprint'ах. Есть такие варианты blueprints или лучше это сделать кодом на C++?  Кодом вроде проще
  (:Pressed
    (Variables|/Script/Engine.CharacterMovementComponent|SetMaxWalkSpeed _charactermovement (Variables|Default|GetHigh_Speed)))
  (:Released
    (Variables|/Script/Engine.CharacterMovementComponent|SetMaxWalkSpeed _charactermovement (Variables|Default|GetSpeed))))

(event Input|AxisEvents|InputAxisMoveRight
  (params (AxisValue :type Float%20%28single-precision%29))
  ;[1 1 1] То что было на уроке
  (Pawn|Input|AddMovementInput (Transformation|GetActorRightVector) AxisValue false))

(event Input|AxisEvents|InputAxisTurn
  (params (AxisValue :type Float%20%28single-precision%29))
  ;[1 1 1] То что было на уроке
  (Pawn|Input|AddControllerYawInput AxisValue))

(event Input|AxisEvents|InputAxisLookUp
  (params (AxisValue :type Float%20%28single-precision%29))
  ;[1 1 1] То что было на уроке
  (Pawn|Input|AddControllerPitchInput AxisValue))

(event Input|AxisEvents|InputAxisMoveForward
  (params (AxisValue :type Float%20%28single-precision%29))
  ;[1 1 1] То что было на уроке
  (Pawn|Input|AddMovementInput (Transformation|GetActorForwardVector) AxisValue false))

(fn ConstructionScript)